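; Character Blueprint that loads a Ready Player Me avatar from a URL in a networked game.
; LoadAvatarServer stores the URL and, with authority, calls LoadAvatarClient, then loads the avatar itself through the ReadyPlayerMe component.
; LoadAvatarClient stores the URL and runs the same load only on remote instances, so the authority does not load twice.
; Load failures print their error message.
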(event `LoadAvatarServer`
  (params (`Avatar URL` :type String))
  (bind _avatarurl (`self.AvatarURL`))
  (set `self.AvatarURL` `Avatar URL`)
  (`/Engine/EditorBlueprintResources/ActorMacros.Switch Has Authority`
    (:`Authority`
      (`|ExecutionSequence`
        (:`then_0`
          (`self.LoadAvatarClient` _avatarurl))
        (:`then_1`
          (`ReadyPlayerMeComponent.LoadNewAvatar` :`self` (`self.ReadyPlayerMeComponent`) :`Url` _avatarurl :`OnLoadFailed` (delegate `OnLoadFailed`) :!label _label))))))

(event `LoadAvatarClient`
  (params (AvatarURL :type String))
  (set `self.AvatarURL` AvatarURL)
  (`/Engine/EditorBlueprintResources/ActorMacros.Switch Has Authority`
    (:`Remote`
      (goto _label))))

(event `OnLoadFailed`
  (params (ErrorMessage :type String))
  (`KismetSystemLibrary.PrintString` ErrorMessage))

(fn `UserConstructionScript`)